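; BP_ItemFactory is an item factory actor that takes on the look of a food or kitchen item, such as a pot, meat or bottle tray, according to its ItemIndex.
; On BeginPlay it copies ItemIndex into FactoryIndex and switches on it to set the Cube component's static mesh, overriding materials for some items.
; Index 4 has no case, and the construction script only calls its parent.
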(event `self.ReceiveBeginPlay`
  (bind _cube (`self.Cube`))
  (bind _cube_2 (`self.Cube`))
  (bind _cube_3 (`self.Cube`))
  (bind _cube_4 (`self.Cube`))
  (bind _output_get (set `self.FactoryIndex` (`self.ItemIndex`)))
  (switch `int` _output_get
    (:`0`
      (`StaticMeshComponent.SetStaticMesh` _cube_3 "/Game/MapAsset/주방기기/low-poly-psx-style-restaurant-props-asset-pack/source/GrillReaperSketchfab_SM_Pot01.GrillReaperSketchfab_SM_Pot01")
      (`PrimitiveComponent.SetMaterial` _cube_3 0 "/Engine/MapTemplates/Materials/BasicAsset02.BasicAsset02"))
    (:`1`
      (`StaticMeshComponent.SetStaticMesh` _cube "/Game/MapAsset/Map/Mesh/Food/SM_BuchuDummy.SM_BuchuDummy")
      (`PrimitiveComponent.SetMaterial` _cube 0 "/Engine/EditorLandscapeResources/SplineEditorMeshMat.SplineEditorMeshMat"))
    (:`2`
      (`StaticMeshComponent.SetStaticMesh` _cube_2 "/Game/MapAsset/Map/Mesh/Food/DadaeGi.DadaeGi")
      (`PrimitiveComponent.SetMaterial` _cube_2 0 "/Game/MapAsset/Map/Materials/Paint_-_Enamel_Glossy__White_.Paint_-_Enamel_Glossy__White_")
      (`PrimitiveComponent.SetMaterial` _cube_2 1 "/Game/MapAsset/Map/Materials/Paint_-_Enamel_Glossy__Red_.Paint_-_Enamel_Glossy__Red_"))
    (:`3`
      (`StaticMeshComponent.SetStaticMesh` (`self.Cube`) "/Game/MapAsset/Map/Mesh/Food/SM_MERGED_MainMeatActor_2.SM_MERGED_MainMeatActor_2"))
    (:`5`
      (`StaticMeshComponent.SetStaticMesh` _cube_4 "/Game/MapAsset/Map/Mesh/SM_DDuk_Dummy.SM_DDuk_Dummy")
      (`PrimitiveComponent.SetMaterial` _cube_4 0 "/Game/MapAsset/Map/Materials/Base01.Base01"))
    (:`6`
      (`StaticMeshComponent.SetStaticMesh` (`self.Cube`) "/Game/MapAsset/Map/Mesh/Bottles_Tray.Bottles_Tray"))))

(fn `UserConstructionScript`
  (`parent.UserConstructionScript`))