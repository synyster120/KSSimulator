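; BP_Item is a holdable item actor whose ItemIndex selects its mesh and materials at BeginPlay, covering Korean soup ingredients and a pot.
; ItemDropInteraction passes the player's HeldItem and HitLocation to DropItem, then clears HeldItem.
; DropItem re-enables collision, detaches the item, lifts it above the target XY, then sweeps it down so it can rest on blocking surfaces.
; It also rotates this actor to the player's forward direction.
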(event `self.ReceiveBeginPlay`
  (bind _cube (`self.Cube`))
  (bind _cube_2 (`self.Cube`))
  (bind _cube_3 (`self.Cube`))
  (bind _cube_4 (`self.Cube`))
  (bind _cube_5 (`self.Cube`))
  ;[1 1 1] Mesh, Material Set
  (switch `int` (`self.ItemIndex`)
    (:`0`
      (`StaticMeshComponent.SetStaticMesh` _cube_3 "/Game/MapAsset/Map/Mesh/Food/Set_Yugsu.Set_Yugsu")
      (`PrimitiveComponent.SetMaterial` _cube_3 0 "/Game/MapAsset/Map/Materials/Material_001.Material_001"))
    (:`1`
      (`StaticMeshComponent.SetStaticMesh` _cube "/Game/MapAsset/Map/Mesh/Food/Set_Buchu.Set_Buchu")
      (`PrimitiveComponent.SetMaterial` _cube 0 "/Game/MapAsset/Map/Texture/textures/01_-_Default.01_-_Default"))
    (:`2`
      (`StaticMeshComponent.SetStaticMesh` _cube_2 "/Game/MapAsset/Map/Mesh/Food/DadaeGi_1.DadaeGi_1")
      (`PrimitiveComponent.SetMaterial` _cube_2 0 "/Game/MapAsset/Map/Materials/Ketchup.Ketchup")
      (`SceneComponent.SetRelativeScale3D` _cube_2 (0.1 0.1 0.1)))
    (:`3`
      (`StaticMeshComponent.SetStaticMesh` _cube_4 "/Game/MapAsset/Map/Mesh/Food/Set_Meat.Set_Meat")
      (`PrimitiveComponent.SetMaterial` _cube_4 0 "/Game/MapAsset/Map/Materials/NewMaterial.NewMaterial")
      (`PrimitiveComponent.SetMaterial` _cube_4 1 "/Game/MapAsset/Map/Materials/NewMaterial.NewMaterial"))
    (:`5`
      (`StaticMeshComponent.SetStaticMesh` _cube_5 "/Game/MapAsset/Map/Mesh/Food/Set_DDukBaeGi.Set_DDukBaeGi")
      (`PrimitiveComponent.SetMaterial` _cube_5 0 "/Game/MapAsset/Map/Materials/Base01.Base01"))))

(event `ItemDropInteraction`
  ;[1 1 1] Drop
  (bind _asbp_kssplayer (cast `/Game/Blueprints/BP_KSSPlayer` (`GameplayStatics.GetPlayerCharacter` 0)))
  (`self.DropItem` (`/Game/Blueprints/BP_KSSPlayer.HeldItem` _asbp_kssplayer) (`/Game/Blueprints/BP_KSSPlayer.HitLocation` _asbp_kssplayer))
  (set `/Game/Blueprints/BP_KSSPlayer.HeldItem` null _asbp_kssplayer))

(fn `DropItem`
  (params (TargetItem :type "Actor Object Reference") (TargetLocation :type "Vector Structure"))
  (locals (LocationVector :type "Vector Structure") (ItemActor :type "Actor Object Reference"))
  (bind _itemactor (`local.ItemActor`))
  (bind _itemactor_2 (`local.ItemActor`))
  (bind _output_get (set `local.ItemActor` TargetItem))
  (bind _output_get_2 (set `local.LocationVector` TargetLocation))
  (`self.SetActorEnableCollision` _itemactor_2 true)
  (`SceneComponent.K2_DetachFromComponent` (`Actor.RootComponent` _itemactor_2) "KeepWorld" "KeepRelative" "KeepRelative" false)
  (bind (_returnvalue_x _returnvalue_y _returnvalue_z) (`KismetMathLibrary.BreakVector` (`self.K2_GetActorLocation` _output_get)))
  ;[1 1 1] XY MoveMent
  (`self.K2_SetActorLocation` _itemactor (`KismetMathLibrary.MakeVector` (.x _output_get_2) (.y _output_get_2) (+ _returnvalue_z 220.0)) false false)
  ;[1 1 1] Z Movement
  (`self.K2_SetActorLocation` _itemactor (`KismetMathLibrary.MakeVector` (.x _output_get_2) (.y _output_get_2) (.z _output_get_2)) true false)
  (`self.K2_SetActorRotation` (`KismetMathLibrary.Conv_VectorToRotator` (`self.GetActorForwardVector` (`GameplayStatics.GetPlayerCharacter` 0)))))

(fn `UserConstructionScript`
  (locals (NewLocalVar :type "PrimaryDataAsset Object Reference")))