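; First-person player character for a food-serving game, handling movement and camera-ray interaction with items, factories, containers, food and customers.
; Interact dispatches on actor tag to grab, drop, combine or serve; negative input deletes unloaded held items.
; GrabItem spawns or returns factory items against GameMode ingredient stock, mounts food on containers and frees customer tables.
; A looping timer reuses the ray to outline targets, clearing every actor's meshes when none is hit.
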(event `self.ReceiveBeginPlay`
  ;[1 1 1] BeginPlay
  (bind _asplayer_controller (cast `PlayerController` (`self.GetController`)))
  (message `EnhancedInputSubsystemInterface.AddMappingContext` (pcsubsystem `EnhancedInputLocalPlayerSubsystem` _asplayer_controller) "/Game/Inputs/IMC_PlayerInput.IMC_PlayerInput" 0 (struct))
  (`KismetSystemLibrary.K2_SetTimer` null "DrawOutLine" 0.1 true))

(event `EnhancedInput|/Game/Inputs/IA_Move`
  (params (ActionValue :type "Vector2D Structure") (ElapsedSeconds :type "Float (double-precision)") (TriggeredSeconds :type "Float (double-precision)") (InputAction :type "InputAction Object Reference" :default "/Game/Inputs/IA_Move.IA_Move"))
  ;[1 1 1] IA_Move
  (:`Triggered`
    (`self.AddMovementInput` (`self.GetActorForwardVector`) ActionValue_X)
    (`self.AddMovementInput` (`self.GetActorRightVector`) ActionValue_Y)))

(event `EnhancedInput|/Game/Inputs/IA_Jump`
  (params (ActionValue :type Boolean) (ElapsedSeconds :type "Float (double-precision)") (TriggeredSeconds :type "Float (double-precision)") (InputAction :type "InputAction Object Reference" :default "/Game/Inputs/IA_Jump.IA_Jump"))
  ;[1 1 1] IA_Jump
  (:`Started`
    (`self.Jump`))
  (:`Canceled`
    (`self.StopJumping`)))

(event `EnhancedInput|/Game/Inputs/IA_Look`
  (params (ActionValue :type "Vector2D Structure") (ElapsedSeconds :type "Float (double-precision)") (TriggeredSeconds :type "Float (double-precision)") (InputAction :type "InputAction Object Reference" :default "/Game/Inputs/IA_Look.IA_Look"))
  ;[1 1 1] IA_Look
  (:`Triggered`
    (`self.AddControllerPitchInput` ActionValue_Y)
    (`self.AddControllerYawInput` ActionValue_X)))

(event `EnhancedInput|/Game/Inputs/IA_Interact`
  (params (ActionValue :type "Float (double-precision)") (ElapsedSeconds :type "Float (double-precision)") (TriggeredSeconds :type "Float (double-precision)") (InputAction :type "InputAction Object Reference" :default "/Game/Inputs/IA_Interact.IA_Interact"))
  ;[1 1 1] Player Interact // RayCast Branches
  (:`Started`
    (`self.PlayerInterAction` ActionValue)))

(fn `DrawOutLine`
  (locals (LocalComp :type "PrimitiveComponent Object Reference") (Local_LastestComponent :type "PrimitiveComponent Object Reference"))
  (bind _tagetactor (`self.TagetActor`))
  (bind _localcomp (`local.LocalComp`))
  (bind _tagetactor_2 (`self.TagetActor`))
  (bind _localcomp_2 (`local.LocalComp`))
  (bind (_raytarget _targetlocation _targetcomponent) (`self.GetRayTarget`))
  (set `local.Local_LastestComponent` (`self.LastestComponent`))
  (`/Engine/EditorBlueprintResources/StandardMacros.IsValid` _tagetactor_2
    (:`Is Valid`
      (bind _tag (`/Game/Blueprints/BP_FuncLibrary.GetActorTag` _tagetactor_2))
      (switch `/Game/E_ActorTags` _tag
        (:`NewEnumerator0`
          (set `local.LocalComp` _targetcomponent :!label _label)
          (`/Engine/EditorBlueprintResources/StandardMacros.IsValid` (`local.Local_LastestComponent`) :!label _label_2
            (:`Is Valid`
              _)
            (:`Is Not Valid`
              (set `self.LastestComponent` (`local.LocalComp`))))
          (if (!= (`local.LocalComp`) (`local.Local_LastestComponent`))
            ;[1 1 1] Branch3: Exchange OutLine Target
            (`/Game/Blueprints/BP_FuncLibrary.TurnOutlineOff` (`local.Local_LastestComponent`))
            (`/Game/Blueprints/BP_FuncLibrary.TurnOutlineOn` _localcomp)
            (set `self.LastestComponent` _localcomp)
            (else
              ;[1 1 1] Branch2 : First Hitted Component -> Draw OutLine, Set LastestComponent
              (`/Game/Blueprints/BP_FuncLibrary.TurnOutlineOn` _localcomp_2)
              (set `self.LastestComponent` _localcomp_2))))
        (:`NewEnumerator5`
          ;[1 1 1] ItemContainerOutLiner
          (for _array_element (`self.K2_GetComponentsByClass` _tagetactor "/Script/Engine.StaticMeshComponent")
            (set `local.LocalComp` _array_element)
            (goto _label_2))
          (for _array_element_2 (`self.GetAttachedActors` _tagetactor true false)
            (for _array_element_3 (`self.K2_GetComponentsByClass` _array_element_2 "/Script/Engine.StaticMeshComponent")
              (set `local.LocalComp` _array_element_3)
              (goto _label_2)))
          (set `self.TagetActor` null))
        (:`NewEnumerator1`
          (goto _label))
        (:`NewEnumerator2`
          (goto _label))
        (:`NewEnumerator3`
          (goto _label))
        (:`NewEnumerator6`
          (goto _label))
        (:`NewEnumerator4`
          ;[1 1 1] Branch_1 : No Hitted Target -> Disable OutLine
          (bind _outactors (`GameplayStatics.GetAllActorsOfClass` "/Script/Engine.Actor" :!label _label_3))
          (for _array_element_4 _outactors
            (for _array_element_5 (`self.K2_GetComponentsByClass` _array_element_4 "/Script/Engine.StaticMeshComponent")
              (`/Game/Blueprints/BP_FuncLibrary.TurnOutlineOff` _array_element_5))))))
    (:`Is Not Valid`
      (goto _label_3))))

(fn `GetRayTarget`
  (returns (RayTarget :type "Actor Object Reference") (TargetLocation :type "Vector Structure") (TargetComponent :type "PrimitiveComponent Object Reference"))
  (locals (bIsItem :type Boolean))
  (bind _firstviewcamera (`self.FirstViewCamera`))
  (bind _returnvalue (`SceneComponent.K2_GetComponentLocation` _firstviewcamera))
  (bind _outhit (`KismetSystemLibrary.LineTraceSingle` _returnvalue (+ _returnvalue (* (`KismetMathLibrary.GetForwardVector` (`SceneComponent.K2_GetComponentRotation` _firstviewcamera)) (`self.RayDistance`))) "TraceTypeQuery3"))
  (bind (_bblockinghit _binitialoverlap _time _distance _location _impactpoint _normal _impactnormal _physmat _hitactor _hitcomponent) (`GameplayStatics.BreakHitResult` _outhit))
  (`/Engine/EditorBlueprintResources/StandardMacros.IsValid` _hitactor
    (:`Is Valid`
      (if (not (== (`PrimitiveComponent.GetCollisionProfileName` _hitcomponent) "Map"))
        (bind _output_get (set `self.TagetActor` _hitactor))
        (return _output_get _impactpoint _hitcomponent)))))

(fn `GrabItem`
  (params (TargetActor :type "Actor Object Reference"))
  (locals (TraceActor :type "Actor Object Reference") (bNotContainer :type Boolean) (AttachedActors :type "Array of Actor Object Reference") (RelativeScale :type "Vector Structure"))
  (bind _traceactor (`local.TraceActor`))
  (bind _helditem (`self.HeldItem`))
  (bind _returnvalue (`KismetMathLibrary.Conv_VectorToTransform` (`self.K2_GetActorLocation`)))
  (bind _rootcomponent (`Actor.RootComponent` (`self.HeldItem`)))
  (set `local.TraceActor` TargetActor)
  (`/Engine/EditorBlueprintResources/StandardMacros.IsValid` _traceactor
    (:`Is Valid`
      (bind _asbp_item_factory (cast `/Game/Blueprints/BP_ItemFactory` _traceactor)
        (:`then`
          (if (`self.bHaveItem`)
            ;[1 1 1] ItemFactory Undo ItemSpawn
            (set `local.AttachedActors` (`self.GetAttachedActors` (`self.HeldItem`) true false))
            (if (== (`KismetArrayLibrary.Array_Length` (`local.AttachedActors`)) 0)
              (bind _asbp_item_factory_2 (cast `/Game/Blueprints/BP_ItemFactory` (`local.TraceActor`)))
              (bind _asbp_item (cast `/Game/Blueprints/BP_Item` (`self.HeldItem`)))
              (bind _itemindex (`/Game/Blueprints/BP_Item.ItemIndex` _asbp_item))
              (if (== (`/Game/Blueprints/BP_ItemFactory.FactoryIndex` _asbp_item_factory_2) _itemindex)
                (if (< _itemindex 4)
                  (bind _asbp_ksgame_mode_base (cast `/Game/Blueprints/BP_KSGameModeBase` (`GameplayStatics.GetGameMode`)))
                  (`KSGameModeBase.SetIngreCount` _asbp_ksgame_mode_base _itemindex 1)
                  (`self.K2_DestroyActor` (`self.HeldItem`))
                  (set `self.bHaveItem` false)
                  (else
                    (`self.K2_DestroyActor` (`self.HeldItem`))
                    (set `self.bHaveItem` false)))))
            (else
              (bind _factoryindex (`/Game/Blueprints/BP_ItemFactory.FactoryIndex` _asbp_item_factory))
              ;[1 1 1] ItemFactory ItemSpawn
              (switch `int` _factoryindex
                (:`0`
                  (bind _asbp_ksgame_mode_base_2 (cast `/Game/Blueprints/BP_KSGameModeBase` (`GameplayStatics.GetGameMode`) :!label _label))
                  (bind _returnvalue_2 (`KSGameModeBase.GetIngreCount` _asbp_ksgame_mode_base_2 _factoryindex))
                  (if (> _returnvalue_2 0)
                    (bind _returnvalue_3 (`|SpawnActorFromClass` "/Game/Blueprints/BP_Item.BP_Item_C" _returnvalue "AlwaysSpawn" "MultiplyWithRoot" null "/Game/DataAssets/DA_IngredientData.DA_IngredientData" _factoryindex "NewEnumerator0" null))
                    (set `self.HeldItem` _returnvalue_3)
                    (bind _asbp_ksgame_mode_base_3 (cast `/Game/Blueprints/BP_KSGameModeBase` (`GameplayStatics.GetGameMode`)))
                    (`KSGameModeBase.SetIngreCount` _asbp_ksgame_mode_base_3 _factoryindex -1)
                    (`self.K2_AttachToComponent` (`self.HeldItem`) (`self.HeldObjectAnchor`) "None" "SnapToTarget" "SnapToTarget" "KeepRelative" false :!label _label_2)
                    (set `self.bHaveItem` true)
                    (`self.SetActorEnableCollision` _helditem false :!label _label_3)
                    (`/Game/Blueprints/BP_FuncLibrary.PrintItemData` _helditem (`local.TraceActor`))))
                (:`1`
                  (goto _label))
                (:`2`
                  (goto _label))
                (:`3`
                  (goto _label))
                (:`5`
                  (bind _returnvalue_4 (`|SpawnActorFromClass` "/Game/Blueprints/BP_Food.BP_Food_C" _returnvalue "AlwaysSpawn" "MultiplyWithRoot" null false "/Game/DataAssets/DA_IngredientData.DA_IngredientData" _factoryindex "NewEnumerator6" null))
                  (set `self.HeldItem` _returnvalue_4)
                  (goto _label_2))
                (:`6`
                  (bind _returnvalue_5 (`|SpawnActorFromClass` "/Game/Blueprints/BP_ItemContainer.BP_ItemContainer_C" _returnvalue "AlwaysSpawn" "MultiplyWithRoot" null 0 "/Game/DataAssets/DA_IngredientData.DA_IngredientData" _factoryindex "NewEnumerator5" null))
                  (set `self.HeldItem` _returnvalue_5)
                  (goto _label_2))))))
        (:`CastFailed`
          (if (`self.bHaveItem`)
            ;[1 1 1] Attach Item To ItemContainer
            (cast `/Game/Blueprints/BP_ItemContainer` (`self.HeldItem`)
              (:`CastFailed`
                (bind _asbp_item_container (cast `/Game/Blueprints/BP_ItemContainer` (`local.TraceActor`)))
                (cast `/Game/Blueprints/BP_Food` (`self.HeldItem`)
                  (:`then`
                    (`self.K2_AttachToComponent` (`self.HeldItem`) (`/Game/Blueprints/BP_ItemContainer.ItemAnchor` _asbp_item_container) "None" "KeepRelative" "KeepRelative" "KeepRelative" false)
                    (`SceneComponent.SetRelativeScale3D` _rootcomponent (0.08 0.08 0.08))
                    (`SceneComponent.K2_SetRelativeLocation` _rootcomponent (0.0 0.0 8.0) false false)
                    (set `self.bHaveItem` false)
                    (set `self.HeldItem` null))
                  (:`CastFailed`
                    (for _array_element (`self.GetAttachedActors` _asbp_item_container true false)
                      (bind _asbp_food (cast `/Game/Blueprints/BP_Food` _array_element))
                      (`/Game/Blueprints/BP_Food.MakeFood` _asbp_food))))))
            (else
              ;[1 1 1] Item Grab
              (bind _asbp_item_container_2 (cast `/Game/Blueprints/BP_ItemContainer` (`local.TraceActor`))
                (:`then`
                  (if (> (`/Game/Blueprints/BP_ItemContainer.SavedTableNum` _asbp_item_container_2) 0)
                    (bind _outactors (`GameplayStatics.GetAllActorsOfClass` "/Game/Blueprints/BP_SpawnCustomer.BP_SpawnCustomer_C"))
                    (for _array_element_2 _outactors
                      (if (== (`/Game/Blueprints/BP_SpawnCustomer.TableNum` _array_element_2) (`/Game/Blueprints/BP_ItemContainer.SavedTableNum` _asbp_item_container_2))
                        (set `/Game/Blueprints/BP_SpawnCustomer.bIsTableEmpty` true _array_element_2)
                        (bind _output_get (set `self.HeldItem` (`local.TraceActor`) :!label _label_4))
                        (bind _output_get_2 (set `local.RelativeScale` (`self.GetActorRelativeScale3D` _output_get)))
                        (`self.K2_AttachToComponent` _output_get (`self.HeldObjectAnchor`) "None" "SnapToTarget" "SnapToTarget" "KeepWorld" false)
                        (`SceneComponent.SetRelativeScale3D` (`Actor.RootComponent` _output_get) _output_get_2)
                        (set `self.bHaveItem` true)
                        (goto _label_3)))
                    (else
                      (goto _label_4))))
                (:`CastFailed`
                  (goto _label_4))))))))))

(fn `PlayerInterAction`
  (params (InputAction :type "Float (double-precision)"))
  (if (> InputAction 0.0)
    (bind (_raytarget _targetlocation) (`self.GetRayTarget`))
    (set `self.HitActor` _raytarget)
    (set `self.HitLocation` _targetlocation)
    ;[1 1 1] Mouse L Button Interaction
    (bind _tag (`/Game/Blueprints/BP_FuncLibrary.GetActorTag` (`self.HitActor`)))
    (switch `/Game/E_ActorTags` _tag
      (:`NewEnumerator0`
        (`self.GrabItem` (`self.HitActor`) :!label _label))
      (:`NewEnumerator5`
        (goto _label))
      (:`NewEnumerator1`
        (goto _label))
      (:`NewEnumerator2`
        (if (`self.bHaveItem`)
          (`/Game/Blueprints/BP_FuncLibrary.Destroy Container` (`self.HeldItem`))
          (set `self.bHaveItem` false)))
      (:`NewEnumerator3`
        (bind _asbp_customer (cast `/Game/Blueprints/BP_Customer` (`self.HitActor`)))
        (`/Game/Blueprints/BP_Customer.CustomerInteract` _asbp_customer))
      (:`NewEnumerator6`
        (if (`self.bHaveItem`)
          (bind _tag_2 (`/Game/Blueprints/BP_FuncLibrary.GetActorTag` (`self.HeldItem`)))
          (switch `/Game/E_ActorTags` _tag_2
            (:`NewEnumerator0`
              (bind _asbp_food (cast `/Game/Blueprints/BP_Food` (`self.HitActor`)))
              (`/Game/Blueprints/BP_Food.MakeFood` _asbp_food)))
          (else
            (goto _label))))
      (:`NewEnumerator4`
        (if (`self.bHaveItem`)
          (`/Engine/EditorBlueprintResources/StandardMacros.IsValid` (`self.HitActor`)
            (:`Is Valid`
              (`/Engine/EditorBlueprintResources/StandardMacros.IsValid` (`self.TagetActor`)
                (:`Is Valid`
                  (bind _asbp_item (cast `/Game/Blueprints/BP_Item` (`self.HeldItem`)))
                  (`/Game/Blueprints/BP_Item.ItemDropInteraction` _asbp_item)
                  (set `self.TagetActor` null)
                  (set `self.bHaveItem` false))))))))
    (else
      ;[1 1 1] Mouse R Button Interaction// Delete Held Item
      (if (`self.bHaveItem`)
        (if (== (`KismetArrayLibrary.Array_Length` (`self.GetAttachedActors` (`self.HeldItem`) true false)) 0)
          (`self.K2_DestroyActor` (`self.HeldItem`))
          (set `self.bHaveItem` false))))))

(fn `UserConstructionScript`)