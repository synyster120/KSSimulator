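; Blueprint function library of shared helpers for items, customers, item factories and containers.
; It resolves an actor's tag from item or customer casts with a default fallback, and destroys containers along with directly attached actors.
; Outline helpers toggle custom depth and stencil for highlighting, and another forces hidden components visible.
; A debug printer shows item names matching the hit factory's index, though its non-item branch reads the failed cast.
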(fn `Destroy Container`
  (params (Container :type "Actor Object Reference"))
  (locals (AttachedActors :type "Array of Actor Object Reference"))
  (bind _output_get (set `local.AttachedActors` (`Actor.GetAttachedActors` Container true false)))
  (for _array_element _output_get
    (`Actor.K2_DestroyActor` _array_element))
  (`Actor.K2_DestroyActor` Container))

(fn `DetVisibility`
  (params (Comp :type "StaticMeshComponent Object Reference"))
  (if (not (`SceneComponent.IsVisible` Comp))
    (`SceneComponent.SetVisibility` Comp true false)))

(fn `GetActorTag`
  (params (TargetActor :type "Actor Object Reference"))
  (returns (Tag :type "/Game/E_ActorTags Enum"))
  (locals (GotTag :type "/Game/E_ActorTags Enum"))
  (bind _asbp_item (cast `/Game/Blueprints/BP_Item` TargetActor)
    (:`then`
      (set `local.GotTag` (`/Game/Blueprints/BP_Item.Tag` _asbp_item)))
    (:`CastFailed`
      (bind _asbp_customer (cast `/Game/Blueprints/BP_Customer` TargetActor)
        (:`then`
          (set `local.GotTag` (`/Game/Blueprints/BP_Customer.Tag` _asbp_customer)))
        (:`CastFailed`
          (set `local.GotTag` "NewEnumerator4")))))
  (return (`local.GotTag`)))

(fn `PrintItemData`
  (params (TargetItem :type "Actor Object Reference") (HitObject :type "Actor Object Reference"))
  (locals (Item :type "Actor Object Reference") (HitTarget :type "Actor Object Reference"))
  (bind _output_get (set `local.Item` TargetItem))
  (set `local.HitTarget` HitObject)
  (bind _asbp_item (cast `/Game/Blueprints/BP_Item` _output_get)
    (:`then`
      (bind _asbp_item_factory (cast `/Game/Blueprints/BP_ItemFactory` (`local.HitTarget`)))
      (bind _items (`Ingredient.Items` (`/Game/Blueprints/BP_Item.ItemStruct` _asbp_item)))
      (for (_array_element _array_index) _items
        (if (== _array_index (`/Game/Blueprints/BP_ItemFactory.FactoryIndex` _asbp_item_factory))
          (`KismetSystemLibrary.PrintText` null (`KismetTextLibrary.Conv_StringToText` (`.Name` (break `IngredientInfo` _array_element)))))))
    (:`CastFailed`
      (for (_array_element_2 _array_index_2) _items
        (if (== _array_index_2 (`/Game/Blueprints/BP_Item.ItemIndex` _asbp_item))
          (`KismetSystemLibrary.PrintText` null (`KismetTextLibrary.Conv_StringToText` (`.Name` (break `IngredientInfo` _array_element_2)))))))))

(fn `TurnOutlineOff`
  (params (TargetComp :type "PrimitiveComponent Object Reference"))
  (`/Engine/EditorBlueprintResources/StandardMacros.IsValid` TargetComp
    (:`Is Valid`
      (`PrimitiveComponent.SetRenderCustomDepth` TargetComp false)
      (`PrimitiveComponent.SetCustomDepthStencilValue` TargetComp 0))))

(fn `TurnOutlineOn`
  (params (TargetComp :type "PrimitiveComponent Object Reference"))
  (`/Engine/EditorBlueprintResources/StandardMacros.IsValid` TargetComp
    (:`Is Valid`
      (`PrimitiveComponent.SetRenderCustomDepth` TargetComp true)
      (`PrimitiveComponent.SetCustomDepthStencilValue` TargetComp 1))))