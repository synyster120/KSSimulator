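; BP_Food is a dish the player assembles from ingredients: soup, buchu, dadegi and meat.
; All child components of Cube start hidden at BeginPlay.
; MakeFood maps the ItemIndex of the player's held BP_Item to an ingredient component for a visibility change, then calls IngredientAdded.
; IngredientAdded destroys the held item, clears HaveItem and sets IsAllFinished according to whether every child of Cube is visible.
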(event `self.ReceiveBeginPlay`
  (bind _output_get (set `self.CompList` (`SceneComponent.GetChildrenComponents` (`self.Cube`) false)))
  (for _array_element _output_get
    (`SceneComponent.SetVisibility` _array_element false false)))

(event `MakeFood`
  (bind _asbp_kssplayer (cast `/Game/Blueprints/BP_KSSPlayer` (`GameplayStatics.GetPlayerCharacter` 0)))
  (bind _asbp_item (cast `/Game/Blueprints/BP_Item` (`/Game/Blueprints/BP_KSSPlayer.HeldItem` _asbp_kssplayer)))
  (switch `int` (`/Game/Blueprints/BP_Item.ItemIndex` _asbp_item)
    (:`0`
      (`/Game/Blueprints/BP_FuncLibrary.DetVisibility` (`self.Soup`)))
    (:`1`
      (`/Game/Blueprints/BP_FuncLibrary.DetVisibility` (`self.Buchu`)))
    (:`2`
      (`/Game/Blueprints/BP_FuncLibrary.DetVisibility` (`self.Dadegi`)))
    (:`3`
      (`/Game/Blueprints/BP_FuncLibrary.DetVisibility` (`self.Meat`))))
  (`self.IngredientAdded`))

(event `IngredientAdded`
  (bind _asbp_kssplayer (cast `/Game/Blueprints/BP_KSSPlayer` (`GameplayStatics.GetPlayerCharacter` 0)))
  (`self.K2_DestroyActor` (`/Game/Blueprints/BP_KSSPlayer.HeldItem` _asbp_kssplayer))
  (set `/Game/Blueprints/BP_KSSPlayer.bHaveItem` false _asbp_kssplayer)
  (bind _output_get (set `self.CompList` (`SceneComponent.GetChildrenComponents` (`self.Cube`) false)))
  (for _array_element _output_get
    (if (`SceneComponent.IsVisible` _array_element)
      (set `self.bIsAllFinished` true)
      (else
        (set `self.bIsAllFinished` false)
        (break)))))

(fn `UserConstructionScript`
  (`parent.UserConstructionScript`))