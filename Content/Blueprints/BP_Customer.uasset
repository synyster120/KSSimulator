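; Restaurant customer that orders at its table, eats the food the player serves, pays and leaves.
; Interaction advances a state enum mirrored to the anim instance, registering an order with the OrderManager and closing it when finished, unused food is served.
; After eating, the tray detaches as used dishes with food hidden, then the customer pays and destroys itself.
; Tick accumulates time for the rating, which reaches the game mode only at 30 seconds or less.
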(event `UpdateRating`
  (if (> (`self.SpentTime`) 50.0)
    (set `self.Rating` -0.2)
    (elif (> (`self.SpentTime`) 30.0)
      (set `self.Rating` 0.0)
      (else
        (bind _asbp_ksgame_mode_base (cast `/Game/Blueprints/BP_KSGameModeBase` (`GameplayStatics.GetGameMode`)))
        (`KSGameModeBase.SetRating` _asbp_ksgame_mode_base (`self.Rating`))))))

(event `self.ReceiveTick`
  (params (DeltaSeconds :type "Float (single-precision)"))
  ;[1 1 1] Comment
  (set `self.SpentTime` (+ DeltaSeconds (stale `self.ReceiveBeginPlay` _output_get))))

(event `self.ReceiveBeginPlay`
  ;[1 1 1] Comment
  (`self.SetState` "NewEnumerator0")
  (bind _output_get (set `self.SpentTime` 0.0))
  (bind _outactors (`GameplayStatics.GetAllActorsOfClass` "/Game/Blueprints/BP_SpawnCustomer.BP_SpawnCustomer_C"))
  (for _array_element _outactors
    (if (== (`/Game/Blueprints/BP_SpawnCustomer.TableNum` _array_element) (`self.SpawnerNum`))
      (set `self.SpawnerActor` _array_element))))

(event `CustomerInteract`
  (bind _asbp_kssplayer (cast `/Game/Blueprints/BP_KSSPlayer` (`GameplayStatics.GetPlayerCharacter` 0)))
  (switch `/Game/E_CustomerState` (`self.State`)
    (:`NewEnumerator0`
      ;[1 1 1] Before Ordering Interact
      (`self.SetState` "NewEnumerator1")
      (bind _asksgame_mode_base (cast `KSGameModeBase` (`GameplayStatics.GetGameMode`)))
      (bind _output_get (set `self.CurrentOrder` (`KSGameModeBase.OrderManager` _asksgame_mode_base)))
      (bind _returnvalue (`OrderManager.OrderIn` _output_get (`self.SpawnerNum`) 0))
      (set `self.OrderNum` _returnvalue))
    (:`NewEnumerator1`
      ;[1 1 1] After Ordering Interact
      (if (`/Game/Blueprints/BP_KSSPlayer.bHaveItem` _asbp_kssplayer)
        (bind _helditem (`/Game/Blueprints/BP_KSSPlayer.HeldItem` _asbp_kssplayer))
        (for _array_element (`self.GetAttachedActors` _helditem true false)
          (bind _asbp_food (cast `/Game/Blueprints/BP_Food` _array_element))
          (if (`/Game/Blueprints/BP_Food.bIsAllFinished` _asbp_food)
            (if (not (`/Game/Blueprints/BP_Food.bUsedDish` _asbp_food))
              (`self.SetState` "NewEnumerator2")
              (bind _output_get_2 (set `self.Food` _helditem))
              (`self.K2_AttachToComponent` _output_get_2 (`/Game/Blueprints/BP_SpawnCustomer.TrayAnchor` (`self.SpawnerActor`)) "None" "KeepRelative" "KeepRelative" "KeepRelative" true)
              (set `/Game/Blueprints/BP_KSSPlayer.bHaveItem` false _asbp_kssplayer)
              (`OrderManager.OrderOut` (`self.CurrentOrder`) (`self.OrderNum`))
              (`self.EatingDone`))))))))

(event `EatingDone`
  (bind _food (`self.Food`))
  ;[1 1 1] Eating Done
  (`KismetSystemLibrary.Delay` 3.0)
  (`self.SetState` "NewEnumerator0")
  (`SceneComponent.K2_DetachFromComponent` (`Actor.RootComponent` (`self.Food`)) "KeepWorld" "KeepWorld" "KeepRelative" true)
  (`self.SetActorEnableCollision` _food true)
  (bind _asbp_item_container (cast `/Game/Blueprints/BP_ItemContainer` _food))
  (`SceneComponent.SetVisibility` (`/Game/Blueprints/BP_ItemContainer.StaticMesh` _asbp_item_container) false false)
  (`SceneComponent.SetVisibility` (`/Game/Blueprints/BP_ItemContainer.StaticMesh1` _asbp_item_container) false false)
  (set `/Game/Blueprints/BP_ItemContainer.SavedTableNum` (`self.SpawnerNum`) _asbp_item_container)
  (for _array_element (`self.GetAttachedActors` (`self.Food`) true false)
    (bind _asbp_food (cast `/Game/Blueprints/BP_Food` _array_element))
    (for _array_element_2 (`SceneComponent.GetChildrenComponents` (`/Game/Blueprints/BP_Item.Cube` _asbp_food) false)
      (`SceneComponent.SetVisibility` _array_element_2 false false))
    (set `/Game/Blueprints/BP_Food.bUsedDish` true _asbp_food)
    (set `/Game/Blueprints/BP_SpawnCustomer.bIsTableEmpty` false (`self.SpawnerActor`))
    ;[1 1 1] Finish Interact
    (`KismetSystemLibrary.Delay` 5.0)
    (bind _asksgame_mode_base (cast `KSGameModeBase` (`GameplayStatics.GetGameMode`)))
    (`KSGameModeBase.SetMoney` _asksgame_mode_base (`self.Pay`))
    (`self.UpdateRating`)
    (`self.K2_DestroyActor`)))

(fn `SetState`
  (params (State :type "/Game/E_CustomerState Enum" :default "NewEnumerator0"))
  (bind _output_get (set `self.State` State))
  (bind _asanim_customer (cast `/Game/Blueprints/Anim_Customer` (`SkeletalMeshComponent.GetAnimInstance` (`self.Mesh`))))
  (`/Game/Blueprints/Anim_Customer.SetAnimationState` _asanim_customer _output_get))

(fn `UserConstructionScript`)