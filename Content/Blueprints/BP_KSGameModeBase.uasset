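; Game mode that periodically spawns customers at free tables.
; On BeginPlay it starts a looping timer with a random interval that shortens as CurrentRating rises, rolled only once, so later rating updates leave it unchanged.
; Each tick refreshes CurrentRating, then finds the first BP_SpawnCustomer with an empty table and no valid customer.
; It spawns a BP_Customer there, facing the spawner's arrow, passes the table number and sets its initial state.
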(event `self.ReceiveBeginPlay`
  (bind _currentrating (`self.CurrentRating`))
  (`KismetSystemLibrary.K2_SetTimerDelegate` (delegate `SpawnCustomer`) (`KismetMathLibrary.RandomFloatInRange` (- 22.0 (* 3.0 _currentrating)) (- 27.0 (* 3.0 _currentrating))) true))

(event `SpawnCustomer`
  (bind _returnvalue (`self.GetRating`))
  (set `self.CurrentRating` _returnvalue)
  (bind _outactors (`GameplayStatics.GetAllActorsOfClass` "/Game/Blueprints/BP_SpawnCustomer.BP_SpawnCustomer_C"))
  (for _array_element _outactors
    (`/Engine/EditorBlueprintResources/StandardMacros.IsValid` (`/Game/Blueprints/BP_SpawnCustomer.CurrentCustomer` _array_element)
      (:`Is Not Valid`
        (if (`/Game/Blueprints/BP_SpawnCustomer.bIsTableEmpty` _array_element)
          (set `self.FitSpawner` _array_element)
          (break)))))
  (`/Engine/EditorBlueprintResources/StandardMacros.IsValid` (`self.FitSpawner`)
    (:`Is Valid`
      (bind _returnvalue_2 (`|SpawnActorFromClass` "/Game/Blueprints/BP_Customer.BP_Customer_C" (`KismetMathLibrary.MakeTransform` (`self.K2_GetActorLocation` (`self.FitSpawner`)) (`KismetMathLibrary.Conv_VectorToRotator` (`SceneComponent.GetForwardVector` (`/Game/Blueprints/BP_SpawnCustomer.Arrow` (`self.FitSpawner`))))) "Undefined" "MultiplyWithRoot" null "NewEnumerator3" (`/Game/Blueprints/BP_SpawnCustomer.TableNum` (`self.FitSpawner`)) null 0.0 0.0 null))
      (bind _output_get (set `/Game/Blueprints/BP_SpawnCustomer.CurrentCustomer` _returnvalue_2 (`self.FitSpawner`)))
      (set `/Game/Blueprints/BP_Customer.State` "NewEnumerator0" _output_get)
      (set `self.FitSpawner` null))))

(fn `UserConstructionScript`)