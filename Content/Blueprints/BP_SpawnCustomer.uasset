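; Spawner actor that periodically spawns a customer for its table.
; On BeginPlay it reads the current rating from the KS game mode and starts a looping timer whose random interval shortens as the rating rises, plus a per-spawner delay.
; Each tick of the timer spawns a customer along the arrow's facing, passing the table number, only if none is active and the table is empty.
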(event `self.ReceiveBeginPlay`
  (bind _currentrating (`self.CurrentRating`))
  (bind _asbp_ksgame_mode_base (cast `/Game/Blueprints/BP_KSGameModeBase` (`GameplayStatics.GetGameMode`)))
  (bind _returnvalue (`KSGameModeBase.GetRating` _asbp_ksgame_mode_base))
  (set `self.CurrentRating` _returnvalue)
  (`KismetSystemLibrary.K2_SetTimerDelegate` (delegate `SpawnCustomer`) (+ (`KismetMathLibrary.RandomFloatInRange` (- 30.0 (* 5.0 _currentrating)) (- 45.0 (* 5.0 _currentrating))) (`self.OwnDelay`)) true))

(event `SpawnCustomer`
  (`/Engine/EditorBlueprintResources/StandardMacros.IsValid` (`self.CurrentCustomer`)
    (:`Is Not Valid`
      (if (`self.bIsTableEmpty`)
        (bind _returnvalue (`|SpawnActorFromClass` "/Game/Blueprints/BP_Customer.BP_Customer_C" (`KismetMathLibrary.MakeTransform` (`self.K2_GetActorLocation`) (`KismetMathLibrary.Conv_VectorToRotator` (`SceneComponent.GetForwardVector` (`self.Arrow`)))) "Undefined" "MultiplyWithRoot" null "NewEnumerator3" (`self.TableNum`) null))
        (bind _output_get (set `self.CurrentCustomer` _returnvalue))
        (set `/Game/Blueprints/BP_Customer.State` "NewEnumerator0" _output_get)))))

(fn `UserConstructionScript`)